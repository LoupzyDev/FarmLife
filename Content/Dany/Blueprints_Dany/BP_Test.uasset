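; BP_Test is a collectible, apparently an animal, that the player pulls in with a left click while in range.
; Sphere overlap with BP_FirstPersonCharacter caches the character and enables the actor's input, and leaving disables it.
; A click plays the AttractionNormalised timeline, lerping the Cube from its current location toward the character's live position without sweep.
; On finish it calls CollectedAnimals on the character and destroys itself.
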(event `Key|LeftMouseButton`
  (params (Key :type "Key Structure"))
  ;[1 1 1] Atraer Animales con Click
  (:`Pressed`
    (bind (_direction _distance) (`Timeline|Attraction(Normalised)`)
      (:`Update`
        (`SceneComponent.K2_SetWorldLocation` (`self.Cube`) (`KismetMathLibrary.VLerp` (`SceneComponent.K2_GetComponentLocation` (`self.Cube`)) (`self.K2_GetActorLocation` (stale `self.Sphere.OnComponentBeginOverlap` _asbp_first_person_character)) _distance) false false))
      (:`Finished`
        (`/Game/Dany/Blueprints_Dany/BP_FirstPersonCharacter.CollectedAnimals` (stale `self.Sphere.OnComponentBeginOverlap` _asbp_first_person_character))
        (`self.K2_DestroyActor`)))))

(event `self.Sphere.OnComponentBeginOverlap`
  (params (OverlappedComponent :type "PrimitiveComponent Object Reference") (OtherActor :type "Actor Object Reference") (OtherComp :type "PrimitiveComponent Object Reference") (OtherBodyIndex :type Integer) (bFromSweep :type Boolean) (SweepResult :type "HitResult Structure (by ref)"))
  ;[1 1 1] Atraer Animales con Click
  (bind _asbp_first_person_character (cast `/Game/Dany/Blueprints_Dany/BP_FirstPersonCharacter` OtherActor))
  (`self.EnableInput` (`GameplayStatics.GetPlayerController` 0)))

(event `self.Sphere.OnComponentEndOverlap`
  (params (OverlappedComponent :type "PrimitiveComponent Object Reference") (OtherActor :type "Actor Object Reference") (OtherComp :type "PrimitiveComponent Object Reference") (OtherBodyIndex :type Integer))
  ;[1 1 1] Atraer Animales con Click
  (cast `/Game/Dany/Blueprints_Dany/BP_FirstPersonCharacter` OtherActor)
  (`self.DisableInput` (`GameplayStatics.GetPlayerController` 0)))

(fn `UserConstructionScript`)